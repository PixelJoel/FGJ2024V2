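; Basket actor that tracks which item actors, identified by a BPC_Item component, sit inside its Box trigger.
; An item entering plays a collect sound and Niagara burst, joins ItemsInBasket, and triggers a debug print of the summed item prices.
; OnItemAdded and OnItemRemoved dispatchers broadcast changes with the basket's ID and reference, with the new item included only on addition.
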(event OnComponentBeginOverlap(Box)
  (params (OverlappedComponent :type Primitive%20Component%20Object%20Reference) (OtherActor :type Actor%20Object%20Reference) (OtherComp :type Primitive%20Component%20Object%20Reference) (OtherBodyIndex :type Integer) (bFromSweep :type Boolean) (SweepResult :type Hit%20Result%20Structure%20%28by%20ref%29))
  (Utilities|IsValid (Actor|GetComponentbyClass OtherActor "/Game/Blueprints/BPC_Item.BPC_Item_C")
    (:Is%20Valid
      (Audio|PlaySoundatLocation "/Game/Audio/success_collect.success_collect" (Transformation|GetActorLocation) "0, 0, 0" 1.0 1.0 0.0 0 0 0 0)
      (Niagara|SpawnSystematLocation "/Game/Blueprints/Basket/Burst_System.Burst_System" (Transformation|GetActorLocation))
      (Utilities|Array|Add (Variables|Default|GetItemsInBasket) OtherActor)
      (bind _totalprice1 (CallFunction|CalculatePrice))
      (Development|PrintString (Utilities|String|ToString(Integer) _totalprice1))
      (Default|CallOnItemAdded OtherActor (Variables|Default|GetBasketID) self))))

(event OnComponentEndOverlap(Box)
  (params (OverlappedComponent :type Primitive%20Component%20Object%20Reference) (OtherActor :type Actor%20Object%20Reference) (OtherComp :type Primitive%20Component%20Object%20Reference) (OtherBodyIndex :type Integer))
  (Utilities|IsValid (Actor|GetComponentbyClass OtherActor "/Game/Blueprints/BPC_Item.BPC_Item_C")
    (:Is%20Valid
      (Utilities|Array|RemoveItem (Variables|Default|GetItemsInBasket) OtherActor)
      (Default|CallOnItemRemoved self (Variables|Default|GetBasketID)))))

(event EventBeginPlay)

(event Collision|EventActorBeginOverlap
  (params (OtherActor :type Actor%20Object%20Reference)))

(event EventTick
  (params (DeltaSeconds :type Float%20%28single-precision%29)))

(fn ConstructionScript)

(fn CalculatePrice
  (for _array_element (Variables|Default|GetItemsInBasket)
    (LocalVariables|SetTotalPrice (+ (LocalVariables|GetTotalPrice) (Variables|/Game/Blueprints/BPC_Item.BPC_Item_C|GetPrice (Actor|GetComponentbyClass _array_element "/Game/Blueprints/BPC_Item.BPC_Item_C")))))
  (return (LocalVariables|GetTotalPrice)))