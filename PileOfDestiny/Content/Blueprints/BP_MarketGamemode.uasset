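; Game mode for a timed market round, running it from countdown to end scene.
; BeginPlay creates the in-game UI, fade overlay and countdown, then flags the game in progress and fires the start dispatcher.
; Tick advances the timer and broadcasts time changes, a one-shot midway event and the round end.
; Ending shows a finished widget, fades, switches the view to the EndgameActor and starts its end scene.
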(event EventBeginPlay
  (bind _returnvalue (UserInterface|CreateWidget "/Game/Art/UI/InGameUI.InGameUI_C"))
  (UserInterface|Viewport|AddtoViewport _returnvalue 0)
  (Variables|Default|SetInGameVUI _returnvalue)
  (bind _returnvalue_2 (Game|ConstructObjectfromClass "/Game/Blueprints/StartWidget/FadeFromBlack.FadeFromBlack_C"))
  (UserInterface|Viewport|AddtoViewport _returnvalue_2 99)
  (bind _output_get (Variables|Default|SetFade _returnvalue_2))
  (Default|Fadeto _output_get true)
  (Utilities|FlowControl|Delay 2.0)
  (bind _returnvalue_3 (UserInterface|CreateWidget "/Game/Blueprints/StartWidget/CountDownWIdget.CountDownWIdget_C"))
  (UserInterface|Viewport|AddtoViewport _returnvalue_3 0)
  (Default|Initialize _returnvalue_3)
  (Utilities|FlowControl|Delay 2.0)
  (Variables|Default|SetGameInProgress true)
  (Default|CallOnGameStart))

(event EventTick
  (params (DeltaSeconds :type Float%20%28single-precision%29))
  (bind _fade (Variables|Default|GetFade))
  (if (Variables|Default|GetGameInProgress)
    (bind _output_get (Variables|Default|SetTimer (+ (Variables|Default|GetTimer) DeltaSeconds)))
    (Default|CallTimeChanged _output_get)
    (Utilities|FlowControl|Sequence
      (:then_0
        (if (not (Variables|Default|GetMidwayFlag))
          (if (> _output_get (* (Variables|Default|GetRoundLength) 0.5))
            (Variables|Default|SetMidwayFlag true)
            (Default|CallOnTimerMidway)
            (Development|PrintString "Midway!"))))
      (:then_1
        (if (> _output_get (Variables|Default|GetRoundLength))
          (Variables|Default|SetGameInProgress false)
          (Default|CallOnGameEnded)
          (bind _returnvalue (Game|ConstructObjectfromClass "/Game/Blueprints/StartWidget/FinishedWidget.FinishedWidget_C"))
          (UserInterface|Viewport|AddtoViewport _returnvalue 0)
          (Utilities|FlowControl|Delay 2.0)
          (Default|Fadeto _fade false)
          (Utilities|FlowControl|Delay 2.0)
          (bind _returnvalue_2 (Actor|GetActorOfClass "/Game/Blueprints/EndgameActor.EndgameActor_C"))
          (Default|Fadeto _fade true)
          (Game|Player|SetViewTargetwithBlend (Game|GetPlayerController 0) _returnvalue_2 0.0 "VTBlend_Linear" 0.0 false)
          (Widget|SetVisibility (Variables|Default|GetInGameVUI) "Hidden")
          (Widget|SetVisibility _returnvalue "Hidden")
          (Utilities|FlowControl|Delay 1.0)
          (Default|BeginEndScene _returnvalue_2))))))

(fn ConstructionScript)