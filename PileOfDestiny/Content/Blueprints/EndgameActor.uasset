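; EndgameActor runs the end scene that totals the item prices from two players' baskets on two widget counters.
; BeginEndScene stacks Basket1's items above a spawn point, then spawns a Kapula divider and stacks Basket2's items.
; While working, Tick pushes physics objects inside Box along X like a conveyor.
; Box1 adds each passing item's price to one counter, switching to the other once the Kapula passes.
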(event OnComponentBeginOverlap(Box)
  (params (OverlappedComponent :type Primitive%20Component%20Object%20Reference) (OtherActor :type Actor%20Object%20Reference) (OtherComp :type Primitive%20Component%20Object%20Reference) (OtherBodyIndex :type Integer) (bFromSweep :type Boolean) (SweepResult :type Hit%20Result%20Structure%20%28by%20ref%29))
  (Utilities|Array|Add (Variables|Default|GetObjectsIN) OtherComp))

(event OnComponentEndOverlap(Box)
  (params (OverlappedComponent :type Primitive%20Component%20Object%20Reference) (OtherActor :type Actor%20Object%20Reference) (OtherComp :type Primitive%20Component%20Object%20Reference) (OtherBodyIndex :type Integer))
  (Utilities|Array|RemoveItem (Variables|Default|GetObjectsIN) OtherComp))

(event OnComponentBeginOverlap(Box1)
  (params (OverlappedComponent :type Primitive%20Component%20Object%20Reference) (OtherActor :type Actor%20Object%20Reference) (OtherComp :type Primitive%20Component%20Object%20Reference) (OtherBodyIndex :type Integer) (bFromSweep :type Boolean) (SweepResult :type Hit%20Result%20Structure%20%28by%20ref%29))
  (bind _returnvalue (Actor|GetComponentbyClass OtherActor "/Game/Blueprints/BPC_Item.BPC_Item_C"))
  (bind _price (Variables|/Game/Blueprints/BPC_Item.BPC_Item_C|GetPrice _returnvalue))
  (Utilities|Casting|CastToKapula OtherActor
    (:then
      (Variables|Default|Setkapulaid 1))
    (:CastFailed
      (if (Math|Conversions|ToBoolean(Integer) (Variables|Default|Getkapulaid))
        (Utilities|IsValid _returnvalue
          (:Is%20Valid
            (bind _output_get (Variables|Default|Set1 (+ (Variables|Default|Get1) _price)))
            (bind _ascounter (Utilities|Casting|CastToCounter (UserInterface|GetWidget (Variables|Default|GetCounter2))))
            (Default|SetNumber _ascounter _output_get)))
        (else
          (Utilities|IsValid _returnvalue
            (:Is%20Valid
              (bind _output_get_2 (Variables|Default|Set2 (+ (Variables|Default|Get2) _price)))
              (bind _ascounter_2 (Utilities|Casting|CastToCounter (UserInterface|GetWidget (Variables|Default|GetCounter1))))
              (Default|SetNumber _ascounter_2 _output_get_2))))))))

(event Custom|BeginEndScene
  (bind _items_in_basket (Variables|Default|GetItems%20in%20Basket))
  (Variables|Default|SetWorking true)
  (bind _outactors (Actor|GetAllActorsOfClass "/Game/Blueprints/Basket/Basket.Basket_C"))
  (Utilities|FlowControl|Sequence
    (:then_0
      (if (Math|Conversions|ToBoolean(Integer) (Variables|/Game/Blueprints/Basket/Basket.Basket_C|GetBasketID (Utilities|Array|Get(acopy) _outactors)))
        (Variables|Default|SetBasket1 (Utilities|Array|Get(acopy) _outactors))
        (else
          (Variables|Default|SetBasket2 (Utilities|Array|Get(acopy) _outactors)))))
    (:then_1
      (if (Math|Conversions|ToBoolean(Integer) (Variables|/Game/Blueprints/Basket/Basket.Basket_C|GetBasketID (Utilities|Array|Get(acopy) _outactors 1)))
        (Variables|Default|SetBasket1 (Utilities|Array|Get(acopy) _outactors 1))
        (else
          (Variables|Default|SetBasket2 (Utilities|Array|Get(acopy) _outactors 1)))))
    (:then_2
      (Utilities|FlowControl|Sequence
        (:then_0
          (for _array_element (Variables|/Game/Blueprints/Basket/Basket.Basket_C|GetItemsInBasket (Variables|Default|GetBasket1))
            (Utilities|Array|Add (Variables|Default|GetItems%20in%20Basket) _array_element)))
        (:then_1
          (Utilities|FlowControl|Delay 2.0)
          (Game|SpawnActorfromClass "/Game/Blueprints/Kapula.Kapula_C" (Math|Conversions|ToTransform(Vector) (Transformation|GetWorldLocation (Variables|Default|GetSpawn))) "Undefined" "MultiplyWithRoot" 0 0)
          (Utilities|Array|Clear (Variables|Default|GetItems%20in%20Basket))
          (Utilities|FlowControl|Delay 1.0)
          (for _array_element_2 (Variables|/Game/Blueprints/Basket/Basket.Basket_C|GetItemsInBasket (Variables|Default|GetBasket2))
            (Utilities|Array|Add (Variables|Default|GetItems%20in%20Basket) _array_element_2))))
      (Development|PrintString (Utilities|String|ToString(Integer) (Utilities|Array|Length _items_in_basket)))
      (for (_array_element_3 _array_index) _items_in_basket
        (Development|PrintString (Utilities|GetDisplayName _array_element_3))
        (Transformation|SetWorldLocation (Actor|GetComponentbyClass _array_element_3 "/Script/Engine.PrimitiveComponent") (+ (Transformation|GetWorldLocation (Variables|Default|GetSpawn)) (Math|Vector|MakeVector 0.0 0.0 (* (Math|Conversions|ToFloat(Integer) _array_index) 2e+02))) false true)
        (Transformation|SetWorldRotation (Actor|GetComponentbyClass _array_element_3 "/Script/Engine.PrimitiveComponent") (Math|Random|RandomRotator false) false false)))))

(event EventBeginPlay
  (Utilities|FlowControl|Sequence
    (:then_0
      (bind _ascounter (Utilities|Casting|CastToCounter (UserInterface|GetWidget (Variables|Default|GetCounter1))))
      (Default|SetPlayer _ascounter))
    (:then_1
      (bind _ascounter_2 (Utilities|Casting|CastToCounter (UserInterface|GetWidget (Variables|Default|GetCounter2))))
      (Default|SetPlayer _ascounter_2 1))))

(event Collision|EventActorBeginOverlap
  (params (OtherActor :type Actor%20Object%20Reference)))

(event EventTick
  (params (DeltaSeconds :type Float%20%28single-precision%29))
  (if (Variables|Default|GetWorking)
    (for _array_element (Variables|Default|GetObjectsIN)
      (if (Class|SceneComponent|IsAnySimulatingPhysics _array_element)
        (Physics|AddForce _array_element (Math|Vector|MakeVector (* -1.0 6e+04) 0.0 0.0) "None" false)))))

(fn ConstructionScript)