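; Actor that displays a world-space price widget for an item, following the item's owner and billboarding toward the camera.
; Initialize stores the Item, finds a PrimitiveComponent on its owner and passes the Item to the PriceWidget.
; BeginPlay caches the camera from BP_CameraManager.
; Each Tick moves the actor to that primitive's location and rotates only the widget component to face the camera.
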(event Custom|Initialize
  (params (Item :type BPC%20Item%20Object%20Reference))
  (bind _output_get (Variables|Default|SetItem Item))
  (Variables|Default|SetPrimi (Actor|GetComponentbyClass (Components|GetOwner _output_get) "/Script/Engine.PrimitiveComponent"))
  (bind _asprice_widget (Utilities|Casting|CastToPriceWidget (UserInterface|GetWidget (Variables|Default|GetWidget))))
  (Default|Initialize _asprice_widget Item))

(event EventBeginPlay
  (bind _returnvalue (Actor|GetActorOfClass "/Game/Blueprints/BP_CameraManager.BP_CameraManager_C"))
  (Variables|Default|SetCamera (Variables|/Game/Blueprints/BP_CameraManager.BP_CameraManager_C|GetCamera _returnvalue)))

(event Collision|EventActorBeginOverlap
  (params (OtherActor :type Actor%20Object%20Reference)))

(event EventTick
  (params (DeltaSeconds :type Float%20%28single-precision%29))
  (CallFunction|MovewithOwner))

(fn ConstructionScript)

(fn MovewithOwner
  (Transformation|SetActorLocation (Transformation|GetWorldLocation (Variables|Default|GetPrimi)) false false)
  (Transformation|SetWorldRotation (Variables|Default|GetWidget) (Math|Rotator|FindLookatRotation (Transformation|GetActorLocation) (Transformation|GetWorldLocation (Variables|Default|GetCamera))) false false))