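; Kasa is a pile spawner for the market game that scatters junk and periodically launches discount goods.
; On BeginPlay it binds to BP_MarketGamemode events and spawns random Roina items at random offsets around itself, with the count driven by KasaAmount.
; Game start begins a delayed loop that spawns a random Alennustavara at the Spawn component, shoves it with an impulse and plays a choir sound.
; The game mode's EndPlay clears the Running flag to stop the loop.
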(event Custom|OnGameStart_Event
  (bind _output_get (Variables|Default|SetRunning true))
  (bind _returnvalue (Game|SpawnActorfromClass (.OutItem (Utilities|Array|Random (Variables|Default|GetAlennustavara))) (Transformation|GetWorldTransform (Variables|Default|GetSpawn)) "Undefined" "MultiplyWithRoot" 0 0 :!label _label))
  (Physics|AddImpulse (Actor|GetComponentbyClass _returnvalue "/Script/Engine.PrimitiveComponent") "0.000000,-200000.000000,0.000000" "None" false)
  (Audio|PlaySound2D "/Game/Audio/holy_choir.holy_choir" 1.0 1.0 0.0 0 0)
  (if _output_get
    (Utilities|FlowControl|Delay 1e+01)
    (goto _label)))

(event Custom|OnEndPlay_Event
  (params (Actor :type Actor%20Object%20Reference) (EndPlayReason :type EEndPlayReason%20Enum :default "Destroyed"))
  (Variables|Default|SetRunning false))

(event EventBeginPlay
  (bind _asbp_market_gamemode (Utilities|Casting|CastToBP_MarketGamemode (Game|GetGameMode)))
  (bind _output_get (Variables|Default|SetAs%20BP%20Market%20Gamemode _asbp_market_gamemode))
  (EventDispatchers|AssignOnGameStart _output_get (delegate Custom|OnGameStart_Event))
  (Game|AssignOnEndPlay _output_get (delegate Custom|OnEndPlay_Event))
  (Utilities|FlowControl|Sequence
    (:then_0
      (for _index (range 0 (Variables|Default|GetKasaAmount))
        (Game|SpawnActorfromClass (.OutItem (Utilities|Array|Random (Variables|Default|GetRoina))) (Math|Conversions|ToTransform(Vector) (+ (Transformation|GetActorLocation) (* (Math|Random|RandomUnitVector) 4e+02))) "Undefined" "MultiplyWithRoot" 0 0)))))

(event Collision|EventActorBeginOverlap
  (params (OtherActor :type Actor%20Object%20Reference)))

(event EventTick
  (params (DeltaSeconds :type Float%20%28single-precision%29)))

(fn ConstructionScript)